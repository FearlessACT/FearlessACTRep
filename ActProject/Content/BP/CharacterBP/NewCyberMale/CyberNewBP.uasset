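; CyberNewBP is a player melee combat character with camera-relative movement and look input.
; GetEnemy gathers visible "Enemy" actors within lock range and orders them by camera yaw offset.
; Helpers cover damage math, combat-state checks, priority montages, hit direction, dodge movement, sprint speed and a timed perfect-defend window.
; Many functions, including TakeDamage, Death and LockSwitch, are empty, and the event graph calls none of the helpers.
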(event EventTick
  (params (DeltaSeconds :type Float%20%28single-precision%29)))

(event Input|ActionEvents|InputActionJump
  (params (Key :type Key%20Structure))
  ;[1 1 1] 移动输入
)

(event Input|AxisEvents|InputAxisMoveForward
  (params (AxisValue :type Float%20%28single-precision%29))
  ;[1 1 1] 移动输入
  (Pawn|Input|AddMovementInput (Math|Vector|GetForwardVector (Math|Rotator|MakeRotator 0.0 0.0 (.yaw (Pawn|GetControlRotation :!class /Script/Engine.Pawn)))) AxisValue true))

(event Input|AxisEvents|InputAxisMoveRight
  (params (AxisValue :type Float%20%28single-precision%29))
  ;[1 1 1] 移动输入
  (Pawn|Input|AddMovementInput (Math|Vector|GetRightVector (Math|Rotator|MakeRotator 0.0 0.0 (.yaw (Pawn|GetControlRotation :!class /Script/Engine.Pawn)))) AxisValue true))

(event Input|AxisEvents|InputAxisLookUp
  (params (AxisValue :type Float%20%28single-precision%29))
  ;[1 1 1] 移动输入
  (Pawn|Input|AddControllerPitchInput AxisValue))

(event Input|AxisEvents|InputAxisTurn
  (params (AxisValue :type Float%20%28single-precision%29))
  ;[1 1 1] 移动输入
  (Pawn|Input|AddControllerYawInput AxisValue))

(event Input|MouseEvents|LeftMouseButton
  (params (Key :type Key%20Structure)))

(event Input|KeyboardEvents|LeftShift
  (params (Key :type Key%20Structure)))

(fn ConstructionScript)

(fn GetEnemy
  (bind _localenemies (Variables|Lock|GetLocalEnemies))
  (Utilities|Map|Clear (Variables|Lock|GetEnemies))
  (Utilities|Array|Clear (Variables|Lock|GetCenterRotation))
  (Utilities|Map|Clear (Variables|Lock|GetLocalEnemies))
  (bind _outactors (Actor|GetAllActorswithTag "Enemy"))
  (for _array_element _outactors
    (if (and (CallFunction|DistanceCheck _array_element) (CallFunction|LightOfSightCheck _array_element))
      (if (not (> (Math|Float|Absolute(Float) (- (.yaw (Math|Rotator|FindLookatRotation (Transformation|GetWorldLocation (Variables|Components|GetCamera)) (Transformation|GetActorLocation _array_element))) (.yaw (Math|Rotator|FindLookatRotation (Transformation|GetWorldLocation (Variables|Components|GetCamera)) (Transformation|GetActorLocation))))) 9e+01))
        (Utilities|Map|Add (Variables|Lock|GetLocalEnemies) _array_element (- (.yaw (Math|Rotator|FindLookatRotation (Transformation|GetWorldLocation (Variables|Components|GetCamera)) (Transformation|GetActorLocation _array_element))) (.yaw (Math|Rotator|FindLookatRotation (Transformation|GetWorldLocation (Variables|Components|GetCamera)) (Transformation|GetActorLocation))))))))
  (while (> (Utilities|Map|Length (Variables|Lock|GetLocalEnemies)) 0)
    (bind _values (Utilities|Map|Values _localenemies))
    (bind _keys (Utilities|Map|Keys _localenemies))
    (Utilities|Map|Add (Variables|Lock|GetEnemies) (Utilities|Array|Get(acopy) _keys (.IndexOfMinValue (Math|Float|MinOfFloatArray _values))) (.MinValue (Math|Float|MinOfFloatArray _values)))
    (Utilities|Array|Add (Variables|Lock|GetCenterRotation) (Math|Float|Absolute(Float) (.MinValue (Math|Float|MinOfFloatArray _values))))
    (Utilities|Map|Remove (Variables|Lock|GetLocalEnemies) (Utilities|Array|Get(acopy) _keys (.IndexOfMinValue (Math|Float|MinOfFloatArray _values)))))
  (return (> (Utilities|Map|Length (Variables|Lock|GetEnemies)) 0)))

(fn DistanceCheck
  (params (Actor :type Actor%20Object%20Reference))
  (return (<= (Transformation|GetDistanceTo Actor) (Variables|Lock|GetLockMaxDistance))))

(fn LightOfSightCheck
  (params (Actor :type Actor%20Object%20Reference))
  (bind _returnvalue (Collision|LineTraceForObjects (Transformation|GetActorLocation) (Transformation|GetActorLocation Actor) (Utilities|Array|MakeArray "ObjectTypeQuery1") false 0 "None"))
  (return (not _returnvalue)))

(fn LockSwitch
  (params (IsLeft :type Boolean)))

(fn TakeDamage
  (params (SkillName :type String) (IsCritical :type Boolean) (Attack :type Float%20%28double-precision%29) (location :type Vector) (Enemy :type Enemy%20Parent%20Object%20Reference)))

(fn ComputeDamage
  (params (skill :type Skill%20Table%20Structure) (atk :type Float%20%28double-precision%29) (isCri :type Boolean))
  (bind (_damage _actionvalue _combodamagecorrection _critratecorrection) (Utilities|Struct|BreakSkillTable skill))
  (bind _hero_def (Variables|Attributes|Gethero_def))
  (bind _returnvalue (* _damage _actionvalue))
  (if isCri
    (return (+ (/ (* _returnvalue _critratecorrection) _hero_def) (/ (* atk _critratecorrection) _hero_def)))
    (else
      (return (/ (+ _returnvalue atk) (Variables|Attributes|Gethero_def))))))

(fn Death)

(fn HurtEffect
  (params (NewParam :type Float%20%28double-precision%29)))

(fn PerfectDefend
  (params (NewParam :type Enemy%20Parent%20Object%20Reference) (NewParam1 :type Direction%20Enum :default "NewEnumerator0")))

(fn NormalDefend)

(fn MontagePriorityPlay
  (params (Montage :type Anim%20Montage%20Object%20Reference) (Priority :type Integer))
  (if (>= Priority (Variables|Anim|GetCurrentMontagePriority))
    (Animation|StopAnimMontage (Animation|GetCurrentMontage :!class /Script/Engine.Character))
    (bind _returnvalue (Animation|PlayAnimMontage Montage 1.0 "None"))
    (return _returnvalue)))

(fn ConditionCheck
  (params (avoid :type Boolean) (attack :type Boolean) (defend :type Boolean) (hurt :type Boolean) (death :type Boolean))
  (if avoid
    (LocalVariables|Setavo true)
    (else
      (LocalVariables|Setavo (not (Variables|Avoid|GetIsAvoid)))))
  (if attack
    (LocalVariables|Setatk true)
    (else
      (LocalVariables|Setatk (Variables|Combo|GetCanEnterNextCombo))))
  (if defend
    (LocalVariables|Setdef true)
    (else
      (LocalVariables|Setdef (not (Variables|Defend|GetIsDefend)))))
  (if hurt
    (LocalVariables|Sethur true)
    (else
      (LocalVariables|Sethur (not (Variables|Hurt|GetIsHurt)))))
  (if death
    (LocalVariables|Setdea true)
    (else
      (LocalVariables|Setdea (not (Variables|Default|GetIsDeath)))))
  (return (Math|Boolean|ANDBoolean (LocalVariables|Getavo) (LocalVariables|Getatk) (LocalVariables|Getdef) (LocalVariables|Gethur) (LocalVariables|Getdea))))

(fn SaveWeaponPosition
  (Variables|Attack|SetLastWeaponPosition (Transformation|GetSocketLocation (Variables|Default|GetWeaponForUse) "Begin")))

(fn HurtDirection
  (params (float :type Float%20%28double-precision%29))
  (LocalVariables|Settemp float)
  (if (and (>= (LocalVariables|Gettemp) -45.0) (<= (LocalVariables|Gettemp) 45.0))
    (return "NewEnumerator1")
    (elif (and (>= (LocalVariables|Gettemp) 45.0) (<= (LocalVariables|Gettemp) 135.0))
      (return "NewEnumerator0")
      (elif (and (>= (LocalVariables|Gettemp) 135.0) (<= (LocalVariables|Gettemp) -135.0))
        (return "NewEnumerator2")
        (elif (and (>= (LocalVariables|Gettemp) -135.0) (<= (LocalVariables|Gettemp) -45.0))
          (return "NewEnumerator3")
          (else
            (return "NewEnumerator0")))))))

(fn StepDirection
  (if (and (== (Variables|Avoid|GetInput%20Y) 0.0) (== (Variables|Avoid|GetInput%20X) 0.0))
    (Variables|Avoid|SetCurrentY 1.0)
    (Variables|Avoid|SetCurrentX 0.0)
    (else
      (Variables|Avoid|SetCurrentY (Variables|Avoid|GetInput%20Y))
      (Variables|Avoid|SetCurrentX (Variables|Avoid|GetInput%20X)))))

(fn StepMove
  (bind _returnvalue (Pawn|GetControlRotation :!class /Script/Engine.Pawn))
  (if (Variables|Avoid|GetIsAvoid)
    (Pawn|Input|AddMovementInput (+ (* (Variables|Avoid|GetCurrentX) (Math|Vector|GetRightVector _returnvalue)) (* (Math|Vector|GetForwardVector _returnvalue) (Variables|Avoid|GetCurrentY))) 1.0 false)))

(fn DashStateCheck
  (if (and (Variables|Default|GetSprintKeyDown) (not (Variables|Avoid|GetIsAvoid)))
    (Variables|Move|SetIsSprint true)
    (Variables|/Script/Engine.CharacterMovementComponent|SetMaxWalkSpeed (Variables|Character|GetCharacterMovement) (Variables|Move|GetMaxSprintSpeed))
    (else
      (Variables|Move|SetIsSprint false)
      (Variables|/Script/Engine.CharacterMovementComponent|SetMaxWalkSpeed (Variables|Character|GetCharacterMovement) (Variables|Move|GetMaxSpeed)))))

(fn WeaponCheck)

(fn GetAvoidMontage)